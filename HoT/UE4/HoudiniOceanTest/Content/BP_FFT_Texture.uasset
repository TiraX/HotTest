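; BP_FFT_Texture configures an FFT ocean texture generator and the shared parameters of the ocean material.
; Its construction script copies wind, wave, depth, choppiness, scale and normal strength settings onto the OceanTexture object and assigns it the Height256 and Normal256 textures.
; It also writes height scale, chop, roughness, metallic and ocean color into the MPC_Ocean parameter collection.
; The event graph holds no active logic.
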(fn `UserConstructionScript`
  (bind _oceantexture (`self.OceanTexture`))
  (`|ExecutionSequence`
    (:`then_0`
      (set `OceanTextureComponent.WindSpeed` (`self.WindSpeed`) _oceantexture)
      (set `OceanTextureComponent.WindDirection` (`self.WindDirection`) _oceantexture)
      (set `OceanTextureComponent.WaveHeight` (`self.WaveHeight`) _oceantexture)
      (set `OceanTextureComponent.ShortestWaveLength` (`self.ShortestWave`) _oceantexture)
      (set `OceanTextureComponent.Damp` (`self.Damp`) _oceantexture)
      (set `OceanTextureComponent.Depth` (`self.Depth`) _oceantexture)
      (set `OceanTextureComponent.Choppyness` (`self.Choppyness`) _oceantexture)
      (set `OceanTextureComponent.HeightScale` (`self.HeightScale`) _oceantexture)
      (set `OceanTextureComponent.ChopScale` (`self.ChopScale`) _oceantexture)
      (set `OceanTextureComponent.SpeedScale` (`self.SpeedScale`) _oceantexture)
      (set `OceanTextureComponent.NormalStrength` (`self.NormalStrength`) _oceantexture))
    (:`then_1`
      (`OceanTextureComponent.SetTexture` (`self.OceanTexture`) "/Game/height256.height256" "/Game/normal256.normal256"))
    (:`then_2`
      (`KismetMaterialLibrary.SetScalarParameterValue` "/Game/MPC_Ocean.MPC_Ocean" "HeightScale" (`self.HeightScale`))
      (`KismetMaterialLibrary.SetScalarParameterValue` "/Game/MPC_Ocean.MPC_Ocean" "Chopness" (`self.ChopScale`))
      (`KismetMaterialLibrary.SetScalarParameterValue` "/Game/MPC_Ocean.MPC_Ocean" "Roughness" (`self.Roughness`))
      (`KismetMaterialLibrary.SetScalarParameterValue` "/Game/MPC_Ocean.MPC_Ocean" "Metallic" (`self.Metallic`))
      (`KismetMaterialLibrary.SetVectorParameterValue` "/Game/MPC_Ocean.MPC_Ocean" "OceanColor" (`self.OceanColor`)))))