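; BP_FFT_Test is an actor that appears to test an FFT-based ocean surface.
; Its construction script copies the actor's ocean settings onto the OceanMesh component, covering grid resolution and size, wind, wave shape, depth, damping and choppiness.
; The event graph holds only disabled placeholder events, so the blueprint itself adds no runtime logic.
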(fn `UserConstructionScript`
  (bind _oceanmesh (`self.OceanMesh`))
  (`|ExecutionSequence`
    (:`then_0`
      (set `OceanMeshComponent.GridRes` (`self.GridRes`) _oceanmesh))
    (:`then_1`
      (set `OceanMeshComponent.WindSpeed` (`self.WindSpeed`) _oceanmesh))
    (:`then_2`
      (set `OceanMeshComponent.WindDirection` (`self.WindDirection`) _oceanmesh))
    (:`then_3`
      (set `OceanMeshComponent.WaveHeight` (`self.WaveHeight`) _oceanmesh))
    (:`then_4`
      (set `OceanMeshComponent.ShortestWaveLength` (`self.ShortestWaveLength`) _oceanmesh))
    (:`then_5`
      (set `OceanMeshComponent.Damp` (`self.Damp`) _oceanmesh))
    (:`then_6`
      (set `OceanMeshComponent.Depth` (`self.Depth`) _oceanmesh))
    (:`then_7`
      (set `OceanMeshComponent.Choppyness` (`self.Choppyness`) _oceanmesh))
    (:`then_8`
      (set `OceanMeshComponent.WindAlign` (`self.WindAlign`) _oceanmesh))
    (:`then_9`
      (set `OceanMeshComponent.WaveScale` (`self.WaveScale`) _oceanmesh))
    (:`then_10`
      (set `OceanMeshComponent.GridSize` (`self.GridSize`) _oceanmesh))))